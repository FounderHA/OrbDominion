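; BP_EnemySpawn spawns BP_Enemy orbs around its own location, each given a random name and skin.
; CallInitialSpawnEnemy, when Active, stores the radius and runs SpawnEnemy for the requested count.
; Cube-root scaling of a random distance spreads spawn points uniformly through the sphere's volume.
; Names come from a shrinking pool copied from OrbListName, falling back to "BOT"; skins come from OrbSkinList.
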(event Custom|SetAvailableOrbNames
  (Variables|Default|SetAvailableOrbNames (Variables|/Game/OrbDominion/Core/Data/OrbNames/PDA_OrbListName.PDA_OrbListName_C|GetNames (Variables|Default|GetOrbListName))))

(fn ConstructionScript)

(fn CallInitialSpawnEnemy
  (params (SpawnSkillPickupRadius :type Float%20%28double-precision%29) (InitialSpawnCount :type Integer))
  (if (Variables|Private|GetActive)
    (Variables|Private|SetSpawnRadius SpawnSkillPickupRadius)
    (Variables|Private|SetInitialSpawnCount InitialSpawnCount)
    (for _index (range 0 (- (Variables|Private|GetInitialSpawnCount) 1))
      (CallFunction|SpawnEnemy))))

(fn SpawnEnemy
  (bind _returnvalue (Game|SpawnActorfromClass "/Game/OrbDominion/Enemy/BP_Enemy.BP_Enemy_C" (Math|Transform|MakeTransform (+ (Transformation|GetActorLocation) (* (Math|Random|RandomUnitVector) (* (Math|Float|Power (Math|Random|RandomFloatinRange 0.0 1.0) 0.3333) (Variables|Private|GetSpawnRadius)))) "0, 0, 0" "1.000000,1.000000,1.000000") "Undefined" "MultiplyWithRoot" 0 0))
  (CallFunction|SetRandomOrbName _returnvalue)
  (CallFunction|SetRandomOrbSkin _returnvalue))

(fn SetRandomOrbName
  (params (Orb :type BP%20Enemy%20Object%20Reference))
  (bind _availableorbnames (Variables|Default|GetAvailableOrbNames))
  (bind (_outitem _outindex) (Utilities|Array|Random _availableorbnames))
  (LocalVariables|SetLocalOrbName _outitem)
  (LocalVariables|SetLocalIndex _outindex)
  (if (Utilities|Text|TextIsEmpty (LocalVariables|GetLocalOrbName))
    (LocalVariables|SetLocalOrbName "BOT")
    (else
      (Utilities|Array|RemoveIndex (Variables|Default|GetAvailableOrbNames) (LocalVariables|GetLocalIndex))))
  (Default|SetOrbName Orb (LocalVariables|GetLocalOrbName)))

(fn SetRandomOrbSkin
  (params (Orb :type BP%20Enemy%20Object%20Reference))
  (Default|SetOrbSkin Orb (.OutItem (Utilities|Array|Random (Variables|/Game/OrbDominion/Core/Data/Skin/PDA_SkinList.PDA_SkinList_C|GetSkinListArray (Variables|Default|GetOrbSkinList))))))