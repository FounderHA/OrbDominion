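; BP_OrbGameModePlay is the play game mode for OrbDominion and handles the victory condition.
; On BeginPlay it binds to the OnBotDie event on the GrowthComponent of every BP_OrbBasePawn present in the level.
; Each bot death recounts those pawns; when exactly one remains, it shows WBP_Victory, switches the first player controller to UI-only input and reveals the cursor.
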(event Custom|OnBotDie
  (bind _returnvalue (Game|GetPlayerController 0))
  (bind _outactors (Actor|GetAllActorsOfClass "/Game/OrbDominion/Core/BP_OrbBasePawn.BP_OrbBasePawn_C"))
  (if (== (Utilities|Array|Length _outactors) 1)
    (bind _returnvalue_2 (UserInterface|CreateWidget "/Game/OrbDominion/UI/EndGame/WBP_Victory.WBP_Victory_C" (Game|GetPlayerController 0)))
    (UserInterface|Viewport|AddtoViewport _returnvalue_2 0)
    (Input|SetInputModeUIOnly _returnvalue 0 "DoNotLock" false)
    (Variables|/Script/Engine.PlayerController|SetbShowMouseCursor _returnvalue true)))

(event EventBeginPlay
  (bind _outactors (Actor|GetAllActorsOfClass "/Game/OrbDominion/Core/BP_OrbBasePawn.BP_OrbBasePawn_C"))
  (for _array_element _outactors
    (EventDispatchers|BindEventtoOnBotDie (Variables|/Game/OrbDominion/Core/BP_OrbBasePawn.BP_OrbBasePawn_C|GetGrowth%20Component _array_element) (EventDispatchers|CreateEvent :!event Custom|OnBotDie))))

(fn ConstructionScript)