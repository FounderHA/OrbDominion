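; Game state for Orb Dominion that keeps a live leaderboard of all orb pawns ranked by points.
; On BeginPlay it caches the first player's gameplay HUD and starts a looping 0.1-second timer.
; Each tick of that timer gathers every orb pawn, selection-sorts them by descending GrowthComponent points, stores the result in RankedOrbs and pushes it to the HUD's ranking widget.
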(event EventBeginPlay
  (bind _asbp_orb_gameplay_hud (Utilities|Casting|CastToBP_OrbGameplayHud (HUD|GetHUD (Game|GetPlayerController 0))))
  (Variables|Default|SetBPOrbGameplayHud _asbp_orb_gameplay_hud)
  (Utilities|Time|SetTimerbyFunctionName 0 "UpdateRanking" 0.1 true))

(fn ConstructionScript)

(fn UpdateRanking
  (bind _outactors (Actor|GetAllActorsOfClass "/Game/OrbDominion/Core/BP_OrbBasePawn.BP_OrbBasePawn_C"))
  (bind _allactorsordered (CallFunction|SortbyDescendingSize _outactors))
  (bind _output_get (Variables|Default|SetRankedOrbs _allactorsordered))
  (Default|UpdateRanking (Variables|/Game/OrbDominion/UI/Hud/WBP_GameHud.WBP_GameHud_C|GetWBP_RankedOrbs (Variables|/Game/OrbDominion/Core/Game/BP_OrbGameplayHud.BP_OrbGameplayHud_C|GetWBPGameHud (Variables|Default|GetBPOrbGameplayHud))) _output_get))

(fn SortbyDescendingSize
  (params (AllActors :type Array%20of%20BP%20Orb%20Base%20Pawn%20Object%20References))
  (bind _output_get (LocalVariables|SetLocalWorkingArray AllActors))
  (bind _output_get_2 (LocalVariables|SetLocalCount (Utilities|Array|Length _output_get)))
  (for _index (range 0 (- _output_get_2 2))
    (LocalVariables|Seti _index)
    (LocalVariables|SetLocalLargestValue (Default|GetPoints (Variables|/Game/OrbDominion/Core/BP_OrbBasePawn.BP_OrbBasePawn_C|GetGrowth%20Component (Utilities|Array|Get(acopy) (LocalVariables|GetLocalWorkingArray) (LocalVariables|Geti)))))
    (LocalVariables|SetLocalLargestIndex (LocalVariables|Geti))
    (for _index_2 (range (+ (LocalVariables|Geti) 1) (- (LocalVariables|GetLocalCount) 1))
      (LocalVariables|Setj _index_2)
      (LocalVariables|SetLocalTempValueJ (Default|GetPoints (Variables|/Game/OrbDominion/Core/BP_OrbBasePawn.BP_OrbBasePawn_C|GetGrowth%20Component (Utilities|Array|Get(acopy) (LocalVariables|GetLocalWorkingArray) (LocalVariables|Getj)))))
      (if (> (LocalVariables|GetLocalTempValueJ) (LocalVariables|GetLocalLargestValue))
        (LocalVariables|SetLocalLargestValue (LocalVariables|GetLocalTempValueJ))
        (LocalVariables|SetLocalLargestIndex (LocalVariables|Getj))))
    (if (!= (LocalVariables|GetLocalLargestIndex) (LocalVariables|Geti))
      (LocalVariables|SetLocalTempActor (Utilities|Array|Get(acopy) (LocalVariables|GetLocalWorkingArray) (LocalVariables|Geti)))
      (Utilities|Array|SetArrayElem (LocalVariables|GetLocalWorkingArray) (LocalVariables|Geti) (Utilities|Array|Get(acopy) (LocalVariables|GetLocalWorkingArray) (LocalVariables|GetLocalLargestIndex)))
      (Utilities|Array|SetArrayElem (LocalVariables|GetLocalWorkingArray) (LocalVariables|GetLocalLargestIndex) (LocalVariables|GetLocalTempActor))))
  (return (LocalVariables|GetLocalWorkingArray)))