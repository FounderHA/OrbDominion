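; BP_FoodSpawner is an actor that spawns BP_OrbFood at random points within a sphere around its location.
; SpawnFood scales a random unit vector by SpawnRadius and a cube root of a random fraction, spreading spawns evenly through the volume.
; SpawnOneFood wraps SpawnFood for other callers.
; BeginPlay only checks Active and does nothing; the InitialSpawnCount loop is disconnected, so no initial food spawns.
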(event Custom|SpawnOneFood
  (CallFunction|SpawnFood))

(event EventBeginPlay
  (if (Variables|Default|GetActive)
    _))

(fn ConstructionScript)

(fn SpawnFood
  (Game|SpawnActorfromClass "/Game/OrbDominion/Core/BP_OrbFood.BP_OrbFood_C" (Math|Transform|MakeTransform (+ (Transformation|GetActorLocation) (* (Math|Random|RandomUnitVector) (* (Math|Float|Power (Math|Random|RandomFloatinRange 0.0 1.0) 0.3333) (Variables|Default|GetSpawnRadius)))) "0, 0, 0" "1.000000,1.000000,1.000000") "Undefined" "MultiplyWithRoot" 0 0))