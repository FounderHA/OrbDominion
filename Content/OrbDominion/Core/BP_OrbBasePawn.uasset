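; Base orb pawn that grows in size, forwarding sphere overlaps to its GrowthComponent and reacting to that component's scale changes.
; Size changes apply instantly or through a timeline, updating actor scale, spring arm length and, optionally, a damped max speed that drops with growth.
; Knockback pauses FloatingPawnMovement ticking while a timeline lerps the pawn to a force-offset location without sweeping.
; BeginPlay also creates the sphere's dynamic skin material.
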(event OnComponentBeginOverlap(OrbSphereColision)
  (params (OverlappedComponent :type Primitive%20Component%20Object%20Reference) (OtherActor :type Actor%20Object%20Reference) (OtherComp :type Primitive%20Component%20Object%20Reference) (OtherBodyIndex :type Integer) (bFromSweep :type Boolean) (SweepResult :type Hit%20Result%20Structure%20%28by%20ref%29))
  (Default|HandleOverlap (Variables|Default|GetGrowth%20Component) OtherActor))

(event OnComponentEndOverlap(OrbSphereColision)
  (params (OverlappedComponent :type Primitive%20Component%20Object%20Reference) (OtherActor :type Actor%20Object%20Reference) (OtherComp :type Primitive%20Component%20Object%20Reference) (OtherBodyIndex :type Integer))
  (Default|HandleEndOverlap (Variables|Default|GetGrowth%20Component) OtherActor))

(event Custom|ApplyKnockback
  (params (Force :type Float%20%28double-precision%29) (Direction :type Vector))
  (bind (_knockbackstartlocation _knockbacktargetlocation) (CallFunction|KnockbackDirection Force Direction))
  (Components|Tick|SetComponentTickEnabled (Variables|Default|GetFloatingPawnMovement) false)
  (bind _alpha (Timeline|TL_Knockback Play)
    (:Update
      (Transformation|SetActorLocation (Math|Vector|Lerp(Vector) _knockbackstartlocation _knockbacktargetlocation _alpha) false false))
    (:Finished
      (Components|Tick|SetComponentTickEnabled (Variables|Default|GetFloatingPawnMovement) true))))

(event Custom|OnSizeChanged
  (params (SmoothRefreshSize :type Boolean) (ScaleFactor :type Float%20%28double-precision%29))
  (Private|Size|ResolvScaleFactor ScaleFactor)
  (if SmoothRefreshSize
    (bind _alpha (Timeline|TL_RefreshSizeScale PlayFromStart)
      (:Update
        (Private|Size|SetSmoothSizeScale3DandVelocity _alpha)
        (Private|Size|SetSmoothOrbNameArmLenght _alpha ScaleFactor)))
    (else
      (Private|Size|SetSizeScale3DandVelocity ScaleFactor)
      (CallFunction|SetOrbNameArmLenght ScaleFactor))))

(event EventBeginPlay
  (CallFunction|CreateDynamicMaterial)
  (Private|Movement|SetMaxSpeed)
  (Private|Config|ExecBinds)
  (Variables|Private|Size|SetOriginalTargetArmLength (Variables|/Script/Engine.SpringArmComponent|GetTargetArmLength (Variables|Default|GetSpringArm)))
  (CallFunction|OnSizeChanged false (Variables|/Game/OrbDominion/Core/Components/AC_GrowthComponent.AC_GrowthComponent_C|GetScaleFactor (Variables|Default|GetGrowth%20Component))))

(fn ConstructionScript)

(fn SetArmLengthGoal)

(fn ExecBinds
  (EventDispatchers|BindEventtoOnScaleSizeChanged (Variables|Default|GetGrowth%20Component) (EventDispatchers|CreateEvent :!event Custom|OnSizeChanged)))

(fn SetSmoothSizeScale3DandVelocity
  (params (Alpha :type Float%20%28double-precision%29))
  (bind _scalefactorstart_ (Variables|Private|Size|GetScaleFactorStart%20))
  (bind _scalefactorgoal_ (Variables|Private|Size|GetScaleFactorGoal%20))
  (bind _returnvalue (Math|Float|Lerp _scalefactorstart_ _scalefactorgoal_ Alpha))
  (Transformation|SetActorScale3D (Math|Vector|MakeVector _returnvalue _returnvalue _returnvalue))
  (if (Variables|Private|Movement|GetReduceSpeedOnGrowth)
    (Variables|/Script/Engine.FloatingPawnMovement|SetMaxSpeed (Variables|Default|GetFloatingPawnMovement) (/ (Variables|Public|Movement|GetBaseMoveSpeed%20) (+ 1.0 (* (- _returnvalue 1.0) (Variables|Private|Movement|GetSpeedDamping)))))))

(fn SetSizeScale3DandVelocity
  (params (ScaleFactor :type Float%20%28double-precision%29))
  (Transformation|SetActorScale3D (Math|Vector|MakeVector ScaleFactor ScaleFactor ScaleFactor))
  (if (Variables|Private|Movement|GetReduceSpeedOnGrowth)
    (Variables|/Script/Engine.FloatingPawnMovement|SetMaxSpeed (Variables|Default|GetFloatingPawnMovement) (/ (Variables|Public|Movement|GetBaseMoveSpeed%20) (+ 1.0 (* (- ScaleFactor 1.0) (Variables|Private|Movement|GetSpeedDamping)))))))

(fn ResolvScaleFactor
  (params (ScaleFactorGoal%20 :type Float%20%28double-precision%29))
  (Variables|Private|Size|SetScaleFactorStart%20 (.x (Transformation|GetActorScale3D)))
  (Variables|Private|Size|SetScaleFactorGoal%20 ScaleFactorGoal%20))

(fn SetMaxSpeed
  (Variables|/Script/Engine.FloatingPawnMovement|SetMaxSpeed (Variables|Default|GetFloatingPawnMovement) (Variables|Public|Movement|GetBaseMoveSpeed%20)))

(fn CreateDynamicMaterial
  (bind _returnvalue (Rendering|Material|CreateDynamicMaterialInstance (Variables|Default|GetSphere) 0 0 "None" :!class /Script/Engine.PrimitiveComponent))
  (Variables|Public|Skin|SetSkinDMI _returnvalue))

(fn KnockbackDirection
  (params (Force :type Float%20%28double-precision%29) (Direction :type Vector))
  (LocalVariables|SetLocalKnockbackStartLocation%20 (Transformation|GetActorLocation))
  (LocalVariables|SetLocalKnockbackTargetLocation (+ (LocalVariables|GetLocalKnockbackStartLocation%20) (* Direction Force)))
  (return (LocalVariables|GetLocalKnockbackStartLocation%20) (LocalVariables|GetLocalKnockbackTargetLocation)))

(fn GetParticleSystem
  (return (Variables|Default|GetParticleSystemSpeed) 0 (Variables|Default|GetParticleSystemShield)))

(fn SetSmoothOrbNameArmLenght
  (params (Alpha :type Float%20%28double-precision%29) (ScaleFactor :type Float%20%28double-precision%29))
  (Variables|/Script/Engine.SpringArmComponent|SetTargetArmLength (Variables|Default|GetSpringArm) (Math|Float|Lerp (Variables|/Script/Engine.SpringArmComponent|GetTargetArmLength (Variables|Default|GetSpringArm)) (* (Variables|Private|Size|GetOriginalTargetArmLength) ScaleFactor) Alpha)))

(fn SetOrbNameArmLenght
  (params (ScaleFactor :type Float%20%28double-precision%29))
  (Variables|/Script/Engine.SpringArmComponent|SetTargetArmLength (Variables|Default|GetSpringArm) (* ScaleFactor (Variables|Private|Size|GetOriginalTargetArmLength))))