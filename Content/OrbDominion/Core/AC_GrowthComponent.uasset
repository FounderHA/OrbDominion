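; Growth component that gives its owning actor a point total and lets the larger actor absorb the smaller.
; Points set uniform scale by square root against base points, and reaching zero destroys the owner.
; HandleOverlap picks the absorber, which swallows targets fully inside its sphere at once.
; Partial overlaps start a looping timer that transfers points in chunks until the target is drained or invalid, without rechecking overlap.
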(event Custom|TickAbsorb
  (CallFunction|ExecutTickAbsorve))

(event EventBeginPlay
  (Private|SetMySpere)
  (Private|RefreshSize))

(fn AddPoints
  (params (Amount :type Float%20%28double-precision%29))
  (Variables|Private|Points|SetPoints (+ (Variables|Private|Points|GetPoints) Amount))
  (Private|RefreshSize))

(fn RemovePoints
  (params (Amount :type Float%20%28double-precision%29))
  (bind _output_get (Variables|Private|Points|SetPoints (Math|Float|Max(Float) (- (Variables|Private|Points|GetPoints) Amount) 0.0)))
  (if (<= _output_get 0.0)
    (Private|Die)
    (else
      (Private|RefreshSize))))

(fn RefreshSize
  (bind _points (Variables|Private|Points|GetPoints))
  (bind _basepoints (Variables|Private|Points|GetBasePoints))
  (bind _returnvalue (/ _points _basepoints))
  (bind _returnvalue_2 (Math|Float|Sqrt _returnvalue))
  (Transformation|SetActorScale3D (Components|GetOwner) (Math|Vector|MakeVector _returnvalue_2 _returnvalue_2 _returnvalue_2)))

(fn CanAbsorb
  (params (OtherComponent :type AC%20Growth%20Component%20Object%20Reference))
  (return (> (Variables|Private|Points|GetPoints) (Variables|AC_GrowthComponent_C|GetPoints OtherComponent))))

(fn Die
  (Actor|DestroyActor (Components|GetOwner)))

(fn HandleOverlap
  (params (OtherActor :type Actor%20Object%20Reference))
  (bind _ac_growthcomponent (CallFunction|FindGrowthComponent OtherActor))
  (Utilities|IsValid _ac_growthcomponent
    (:Is%20Valid
      (if (Private|CanAbsorb _ac_growthcomponent)
        (Private|AbsorbOther _ac_growthcomponent)
        (elif (Private|CanAbsorb _ac_growthcomponent self)
          (Private|AbsorbOther _ac_growthcomponent self))))))

(fn AbsorbOther
  (params (TargetGrowth :type AC%20Growth%20Component%20Object%20Reference))
  (bind _points (Variables|AC_GrowthComponent_C|GetPoints TargetGrowth))
  (Utilities|IsValid (Components|GetOwner TargetGrowth)
    (:Is%20Valid
      (Utilities|IsValid TargetGrowth
        (:Is%20Valid
          (Variables|Private|Component|SetAbsorbTarget TargetGrowth)
          (if (Private|IsFullyOverlapping TargetGrowth)
            (Private|AddPoints _points)
            (Private|RemovePoints TargetGrowth _points)
            (else
              (bind _returnvalue (Utilities|Time|SetTimerbyEvent (EventDispatchers|CreateEvent :!event Custom|TickAbsorb) (Variables|Private|Tick|GetAbsorbTickRate) true))
              (Variables|Private|Tick|SetAbsorbTimerHandle _returnvalue))))))))

(fn GetPoints
  (return (Variables|Private|Points|GetPoints)))

(fn SetMySpere
  (Variables|Private|Component|SetMySphere (Actor|GetComponentbyClass (Components|GetOwner) "/Script/Engine.SphereComponent")))

(fn IsFullyOverlapping
  (params (OtherGrowth :type AC%20Growth%20Component%20Object%20Reference))
  (LocalVariables|SetLocalOtherSphere (Actor|GetComponentbyClass (Components|GetOwner OtherGrowth) "/Script/Engine.SphereComponent"))
  (return (<= (Math|Vector|Distance(Vector) (Transformation|GetWorldLocation (Variables|Private|Component|GetMySphere)) (Transformation|GetWorldLocation (LocalVariables|GetLocalOtherSphere))) (- (Components|Sphere|GetScaledSphereRadius (Variables|Private|Component|GetMySphere)) (Components|Sphere|GetScaledSphereRadius (LocalVariables|GetLocalOtherSphere))))))

(fn ExecutTickAbsorve
  (bind _absorbtarget (Variables|Private|Component|GetAbsorbTarget))
  (Utilities|IsValid _absorbtarget
    (:Is%20Valid
      (Utilities|IsValid (Components|GetOwner _absorbtarget)
        (:Is%20Valid
          (if (> (Public|GetPoints (Variables|Private|Component|GetAbsorbTarget)) 0.0)
            (LocalVariables|SetLocalAmount (Math|Float|Min(Float) (Variables|Private|Tick|GetAbsorbAmountPerTick) (Public|GetPoints (Variables|Private|Component|GetAbsorbTarget))))
            (Private|AddPoints (LocalVariables|GetLocalAmount))
            (Private|RemovePoints (Variables|Private|Component|GetAbsorbTarget) (LocalVariables|GetLocalAmount))
            (else
              (Utilities|Time|ClearandInvalidateTimerbyHandle (Variables|Private|Tick|GetAbsorbTimerHandle)))))
        (:Is%20Not%20Valid
          (Utilities|Time|ClearandInvalidateTimerbyHandle (Variables|Private|Tick|GetAbsorbTimerHandle)))))
    (:Is%20Not%20Valid
      (Utilities|Time|ClearandInvalidateTimerbyHandle (Variables|Private|Tick|GetAbsorbTimerHandle)))))