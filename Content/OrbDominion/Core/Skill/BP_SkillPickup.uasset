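; BP_SkillPickup is a world pickup that grants a charge of a randomly chosen skill to an actor that overlaps it.
; On BeginPlay it creates a dynamic material, then picks a random entry from SkillOptions to set its skill type and texture.
; Sphere overlap calls TryGrantCharge on the other actor's skill component.
; Only a successful grant fires the collected notification and destroys the pickup.
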(event OnComponentBeginOverlap(SphereCollision)
  (params (OverlappedComponent :type Primitive%20Component%20Object%20Reference) (OtherActor :type Actor%20Object%20Reference) (OtherComp :type Primitive%20Component%20Object%20Reference) (OtherBodyIndex :type Integer) (bFromSweep :type Boolean) (SweepResult :type Hit%20Result%20Structure%20%28by%20ref%29))
  (bind _ac_skillcomponent (CallFunction|FindSkillComponent OtherActor))
  (Utilities|IsValid _ac_skillcomponent
    (:Is%20Valid
      (bind _success (Default|TryGrantCharge _ac_skillcomponent (Variables|Private|GetCurrentSkillType)))
      (if _success
        (Default|CallOnSkillPickupColected)
        (Actor|DestroyActor)))))

(event EventBeginPlay
  (bind _returnvalue (Rendering|Material|CreateDynamicMaterialInstance (Variables|Default|GetMesh) 0 "/Game/OrbDominion/MaterialLibrary/Skill/MI_SkillPickup.MI_SkillPickup" "None" :!class /Script/Engine.PrimitiveComponent))
  (Variables|Private|SetDynamicMat _returnvalue)
  (CallFunction|RandomizeSkill))

(fn ConstructionScript)

(fn RandomizeSkill
  (LocalVariables|SetLocalRandomSkill (.OutItem (Utilities|Array|Random (Variables|Private|GetSkillOptions))))
  (Variables|Private|SetCurrentSkillType (Variables|/Game/OrbDominion/Core/Data/Skill/PDA/PDA_Skill.PDA_Skill_C|GetSkillType (LocalVariables|GetLocalRandomSkill)))
  (Rendering|Material|SetTextureParameterValue (Variables|Private|GetDynamicMat) "Texture" (Variables|/Game/OrbDominion/Core/Data/Skill/PDA/PDA_Skill.PDA_Skill_C|GetTexture (LocalVariables|GetLocalRandomSkill))))

(fn Initialize)

(fn GetCurrentSkillType
  (return (Variables|Private|GetCurrentSkillType)))