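; BP_SkillSpawner populates a spherical area around itself with BP_SkillPickup actors.
; When Active, CallInitialSpawnSkill stores the radius, count and delay, spawns the initial batch and starts a looping timer at the respawn delay.
; SpawnSkillPickup scales a random unit vector by an approximate cube root of a random value, spreading pickups evenly through the sphere's volume.
; RequestRespawn spawns one additional pickup per call.
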(fn ConstructionScript)

(fn CallInitialSpawnSkill
  (params (SpawnSkillPickupRadius :type Float%20%28double-precision%29) (InitialSpawnCount :type Integer) (RespawnSkillDelay :type Float%20%28double-precision%29))
  (if (Variables|Private|GetActive)
    (Variables|Private|SetSpawnRadius SpawnSkillPickupRadius)
    (Variables|Private|SetInitialSpawnCount InitialSpawnCount)
    (Variables|Private|SetRespawnSkillDelay RespawnSkillDelay)
    (for _index (range 0 (- (Variables|Private|GetInitialSpawnCount) 1))
      (CallFunction|SpawnSkillPickup))
    (bind _returnvalue (Utilities|Time|SetTimerbyEvent (EventDispatchers|CreateEvent :!event RequestRespawn) (Variables|Private|GetRespawnSkillDelay) true))
    (Variables|Private|SetSpawnTimerHandle _returnvalue)))

(fn SpawnSkillPickup
  (Game|SpawnActorfromClass "/Game/OrbDominion/Core/Skill/BP_SkillPickup.BP_SkillPickup_C" (Math|Transform|MakeTransform (+ (Transformation|GetActorLocation) (* (Math|Random|RandomUnitVector) (* (Math|Float|Power (Math|Random|RandomFloatinRange 0.0 1.0) 0.3333) (Variables|Private|GetSpawnRadius)))) "0, 0, 0" "1.000000,1.000000,1.000000") "Undefined" "MultiplyWithRoot" 0 0))

(fn RequestRespawn
  (CallFunction|SpawnSkillPickup))