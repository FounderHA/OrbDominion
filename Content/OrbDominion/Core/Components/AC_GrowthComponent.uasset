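; Actor component for an orb-eating game: tracks points as size and handles absorbing other orbs.
; Points drive square-root scaling and milestone camera-boom updates through dispatchers.
; Overlaps absorb instantly at roughly 80% sphere coverage, otherwise a looping timer transfers percentages from smaller to larger, unless a shielded target drains its unshielded attacker.
; Reaching zero points shows game over for players and destroys other owners.
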(event Custom|TickAbsorb
  (Private|Absorb|ExecutTickAbsorve))

(event Custom|FoodAbsorb
  (params (Value :type Float%20%28double-precision%29))
  (Private|Points|AddPoints Value true))

(event EventBeginPlay
  (Private|Config|SetMySpere)
  (Private|ScaleSize|RefreshSize false)
  (Private|Config|SetCameraBoom))

(fn AddPoints
  (params (Amount :type Float%20%28double-precision%29) (SmoothRefreshSize :type Boolean))
  (Variables|Private|Points|SetPoints (+ (Variables|Private|Points|GetPoints) Amount))
  (bind _scalefactor (Private|ScaleSize|RefreshSize SmoothRefreshSize))
  (Private|Camera|CalculeMilestoneReachedCamera _scalefactor))

(fn RemovePoints
  (params (Amount :type Float%20%28double-precision%29) (SmoothRefreshSize :type Boolean))
  (bind _output_get (Variables|Private|Points|SetPoints (Math|Float|Max(Float) (- (Variables|Private|Points|GetPoints) Amount) 0.0)))
  (if (<= _output_get 0.0)
    (Private|Points|Die)
    (else
      (Private|ScaleSize|RefreshSize SmoothRefreshSize))))

(fn RefreshSize
  (params (SmoothRefreshSize :type Boolean))
  (bind _output_get (LocalVariables|SetLocalScaleFactor (Math|Float|Sqrt (/ (Variables|Private|Points|GetPoints) (Variables|Private|Points|GetBasePoints)))))
  (Variables|Default|SetScaleFactor _output_get)
  (Default|CallOnScaleSizeChanged SmoothRefreshSize (LocalVariables|GetLocalScaleFactor))
  (return (LocalVariables|GetLocalScaleFactor)))

(fn CanAbsorb
  (params (OtherComponent :type AC%20Growth%20Component%20Object%20Reference))
  (return (> (Variables|Private|Points|GetPoints) (Variables|AC_GrowthComponent_C|GetPoints OtherComponent))))

(fn Die
  (bind _returnvalue (Components|GetOwner))
  (bind _returnvalue_2 (Game|GetPlayerController 0))
  (if (not (Variables|Default|GetIsDead))
    (Variables|Default|SetIsDead true)
    (Utilities|IsValid _returnvalue
      (:Is%20Valid
        (bind _aspawn (Utilities|Casting|CastToPawn _returnvalue))
        (if (Pawn|IsPlayerControlled _aspawn)
          (bind _returnvalue_3 (UserInterface|CreateWidget "/Game/OrbDominion/UI/GameOver/WBP_GameOver.WBP_GameOver_C" (Game|GetPlayerController 0)))
          (UserInterface|Viewport|AddtoViewport _returnvalue_3 0)
          (Input|SetInputModeUIOnly _returnvalue_2 0 "DoNotLock" false)
          (Variables|/Script/Engine.PlayerController|SetbShowMouseCursor _returnvalue_2 true)
          (else
            (Actor|DestroyActor (Components|GetOwner))))))))

(fn HandleOverlap
  (params (OtherActor :type Actor%20Object%20Reference))
  (bind _ac_growthcomponent (CallFunction|FindGrowthComponent OtherActor))
  (Utilities|IsValid _ac_growthcomponent
    (:Is%20Valid
      (if (Private|Absorb|CanAbsorb _ac_growthcomponent)
        (Private|Absorb|AbsorbOther _ac_growthcomponent)))))

(fn AbsorbOther
  (params (TargetGrowth :type AC%20Growth%20Component%20Object%20Reference))
  (bind _points (Variables|AC_GrowthComponent_C|GetPoints TargetGrowth))
  (Utilities|IsValid TargetGrowth
    (:Is%20Valid
      (Utilities|IsValid (Components|GetOwner TargetGrowth)
        (:Is%20Valid
          (if (Private|Overlap|IsFullyOverlapping TargetGrowth)
            (Private|Points|AddPoints _points true)
            (Private|Points|RemovePoints TargetGrowth _points false)
            (elif (not (Utilities|Array|ContainsItem (Variables|Private|Component|GetAbsorbTargets) TargetGrowth))
              (Utilities|Array|AddUnique (Variables|Private|Component|GetAbsorbTargets) TargetGrowth)
              (if (not (Utilities|Time|IsTimerActivebyHandle (Variables|Private|Tick|GetAbsorbTimerHandle)))
                (bind _returnvalue (Utilities|Time|SetTimerbyEvent (EventDispatchers|CreateEvent :!event Custom|TickAbsorb) (Variables|Private|Tick|GetAbsorbTickRate) true))
                (Variables|Private|Tick|SetAbsorbTimerHandle _returnvalue)))))))))

(fn GetPoints
  (return (Variables|Private|Points|GetPoints)))

(fn SetMySpere
  (Variables|Private|Component|SetMySphere (Actor|GetComponentbyClass (Components|GetOwner) "/Script/Engine.SphereComponent")))

(fn IsFullyOverlapping
  (params (OtherGrowth :type AC%20Growth%20Component%20Object%20Reference))
  (LocalVariables|SetLocalOtherSphere (Actor|GetComponentbyClass (Components|GetOwner OtherGrowth) "/Script/Engine.SphereComponent"))
  (if (>= (Math|Float|Clamp(Float) (/ (- (+ (Components|Sphere|GetScaledSphereRadius (Variables|Private|Component|GetMySphere)) (Components|Sphere|GetScaledSphereRadius (LocalVariables|GetLocalOtherSphere))) (Math|Vector|Distance(Vector) (Transformation|GetWorldLocation (Variables|Private|Component|GetMySphere)) (Transformation|GetWorldLocation (LocalVariables|GetLocalOtherSphere)))) (* (Components|Sphere|GetScaledSphereRadius (LocalVariables|GetLocalOtherSphere)) 2.0))) 0.8)
    (Development|PrintString "full overlaping" true true "(R=1.000000,G=0.019160,B=0.000000,A=1.000000)" 15.0))
  (return (>= (Math|Float|Clamp(Float) (/ (- (+ (Components|Sphere|GetScaledSphereRadius (Variables|Private|Component|GetMySphere)) (Components|Sphere|GetScaledSphereRadius (LocalVariables|GetLocalOtherSphere))) (Math|Vector|Distance(Vector) (Transformation|GetWorldLocation (Variables|Private|Component|GetMySphere)) (Transformation|GetWorldLocation (LocalVariables|GetLocalOtherSphere)))) (* (Components|Sphere|GetScaledSphereRadius (LocalVariables|GetLocalOtherSphere)) 2.0))) 0.8)))

(fn ExecutTickAbsorve
  (bind _points (Variables|Private|Points|GetPoints))
  (bind _points_2 (Variables|Private|Points|GetPoints))
  ;[0.15 0.15 0.15 0.5] Loop
  ;
  ; Faz o loop em todos os atores no Overlap e set variaveis locais
  (bind (_arrayindex _arrayelement) (Utilities|Array|ReverseforEachLoop (Variables|Private|Component|GetAbsorbTargets))
    (:LoopBody
      (LocalVariables|SetLocalElementIndex _arrayindex)
      (LocalVariables|SetLocalElement _arrayelement)
      ;[0.15 0.15 0.15 0.5] Validação
      ;
      ; Confirma que o Ator e o ActorComponent são validos. Se não for valido remove do Array
      (Utilities|IsValid (LocalVariables|GetLocalElement)
        (:Is%20Valid
          (Utilities|IsValid (Components|GetOwner (LocalVariables|GetLocalElement))
            (:Is%20Valid
              ;[0.15 0.15 0.15 0.5] CheckShield
              ;
              ; verificação de shield ativo
              (if (Public|Gets|GetHasShieldActive (LocalVariables|GetLocalElement))
                (if (Variables|Private|Shield|GetHasShieldActive)
                  (if (not (== (Variables|Private|Points|GetPoints) (Public|Gets|GetPoints (LocalVariables|GetLocalElement)))) :!label _label
                    (if (> (Variables|Private|Points|GetPoints) (Public|Gets|GetPoints (LocalVariables|GetLocalElement)))
                      ;[0.15 0.15 0.15 0.5] Fully Overlapping
                      ;
                      ; Verifica se o Player fez o Overlap completo no Alvo
                      ;
                      ; True: Absorve completamente em um Tick
                      ; False: Aborve o AmountPerTick
                      (if (Private|Overlap|IsFullyOverlapping (LocalVariables|GetLocalElement))
                        ;[0.15 0.15 0.15 0.5] Absorve Fully
                        ;
                        ; Adiciona os pontos em Self e Remove os pontos no Target e Remove o index do Array
                        (Private|Points|AddPoints (Variables|AC_GrowthComponent_C|GetPoints (LocalVariables|GetLocalElement)) true)
                        (Private|Points|RemovePoints (LocalVariables|GetLocalElement) (Variables|AC_GrowthComponent_C|GetPoints (LocalVariables|GetLocalElement)) false)
                        (Utilities|Array|RemoveIndex (Variables|Private|Component|GetAbsorbTargets) (LocalVariables|GetLocalElementIndex))
                        (else
                          ;[0.15 0.15 0.15 0.5] TickAbsorb
                          ;
                          ; Fas a verificação final se o Point do alvo é maior que 0.
                          ;
                          ; True: Remove o AmountPerTick
                          ; False: Remove o Index
                          (if (> (Public|Gets|GetPoints (LocalVariables|GetLocalElement)) 0.0)
                            (if (<= (Public|Gets|GetPoints (LocalVariables|GetLocalElement)) 1e+01)
                              ;[0.15 0.15 0.15 0.5] Caso a vida do oponent seja menor que 10 e ainda nao tenha feito fullyoverlaping ele ainda assim é consumido de vez
                              (Private|Points|AddPoints (Variables|AC_GrowthComponent_C|GetPoints (LocalVariables|GetLocalElement)) true)
                              (Private|Points|RemovePoints (LocalVariables|GetLocalElement) (Variables|AC_GrowthComponent_C|GetPoints (LocalVariables|GetLocalElement)) true)
                              (Utilities|Array|RemoveIndex (Variables|Private|Component|GetAbsorbTargets) (LocalVariables|GetLocalElementIndex))
                              (else
                                (LocalVariables|SetLocalAmount (Math|Float|Min(Float) (* (Public|Gets|GetPoints (LocalVariables|GetLocalElement)) (Variables|Private|Tick|GetAbsorbPercentAmountPerTick)) (Public|Gets|GetPoints (LocalVariables|GetLocalElement))))
                                (Private|Points|AddPoints (LocalVariables|GetLocalAmount) true)
                                (Private|Points|RemovePoints (LocalVariables|GetLocalElement) (LocalVariables|GetLocalAmount) true)))
                            (else
                              (Utilities|Array|RemoveIndex (Variables|Private|Component|GetAbsorbTargets) (LocalVariables|GetLocalElementIndex))))))
                      (elif (Private|Overlap|IsFullyOverlappingEnemy (LocalVariables|GetLocalElement))
                        (Private|Points|AddPoints (LocalVariables|GetLocalElement) (Variables|Private|Points|GetPoints) true)
                        (Private|Points|RemovePoints (Variables|Private|Points|GetPoints) true)
                        (elif (<= (Variables|Private|Points|GetPoints) 1e+01)
                          (Private|Points|AddPoints (LocalVariables|GetLocalElement) (Variables|AC_GrowthComponent_C|GetPoints (LocalVariables|GetLocalElement)) true)
                          (Private|Points|RemovePoints (Variables|AC_GrowthComponent_C|GetPoints (LocalVariables|GetLocalElement)) true)
                          (else
                            (LocalVariables|SetLocalAmount (Math|Float|Min(Float) (* _points (Variables|Private|Tick|GetAbsorbPercentAmountPerTick)) _points))
                            (Private|Points|AddPoints (LocalVariables|GetLocalElement) (LocalVariables|GetLocalAmount) true)
                            (Private|Points|RemovePoints (LocalVariables|GetLocalAmount) true))))))
                  (elif (Private|Overlap|IsFullyOverlappingEnemy (LocalVariables|GetLocalElement))
                    (Private|Points|AddPoints (LocalVariables|GetLocalElement) (Variables|Private|Points|GetPoints) true)
                    (Private|Points|RemovePoints (Variables|Private|Points|GetPoints) true)
                    (else
                      ;[0.15 0.15 0.15 0.5] TickAbsorb
                      ;
                      ; Fas a verificação final se o Point do alvo é maior que 0.
                      ;
                      ; True: Remove o AmountPerTick
                      ; False: Remove o Index
                      (if (<= (Variables|Private|Points|GetPoints) 1e+01)
                        (Private|Points|AddPoints (LocalVariables|GetLocalElement) (Variables|Private|Points|GetPoints) true)
                        (Private|Points|RemovePoints (Variables|Private|Points|GetPoints) true)
                        (else
                          (LocalVariables|SetLocalAmount (Math|Float|Min(Float) (* _points_2 (Variables|Private|Shield|GetShieldAbsorbAmountPerTick)) _points_2))
                          (Private|Points|AddPoints (LocalVariables|GetLocalElement) (LocalVariables|GetLocalAmount) true)
                          (Private|Points|RemovePoints (LocalVariables|GetLocalAmount) true))))))
                (else
                  (goto _label))))
            (:Is%20Not%20Valid
              (Utilities|Array|RemoveIndex (Variables|Private|Component|GetAbsorbTargets) (LocalVariables|GetLocalElementIndex)))))
        (:Is%20Not%20Valid
          (Utilities|Array|RemoveIndex (Variables|Private|Component|GetAbsorbTargets) (LocalVariables|GetLocalElementIndex)))))
    (:Completed
      ;[0.15 0.15 0.15 0.5] Clear Timer
      ;
      ; Verifica se no Array ainda tem algum elemento. se não tiver para o Timer
      (if (<= (Utilities|Array|Length (Variables|Private|Component|GetAbsorbTargets)) 0)
        (Utilities|Time|ClearandInvalidateTimerbyHandle (Variables|Private|Tick|GetAbsorbTimerHandle))))))

(fn HandleEndOverlap
  (params (OtherActor :type Actor%20Object%20Reference))
  (bind _ac_growthcomponent (CallFunction|FindGrowthComponent OtherActor))
  (Utilities|IsValid _ac_growthcomponent
    (:Is%20Valid
      (Utilities|Array|RemoveItem (Variables|Private|Component|GetAbsorbTargets) _ac_growthcomponent)
      (if (<= (Utilities|Array|Length (Variables|Private|Component|GetAbsorbTargets)) 0)
        (Utilities|Time|ClearandInvalidateTimerbyHandle (Variables|Private|Tick|GetAbsorbTimerHandle))))))

(fn SetCameraBoom
  (bind _output_get (Variables|Private|Component|SetMyCameraBoom (Actor|GetComponentbyClass (Components|GetOwner) "/Script/Engine.SpringArmComponent")))
  (Variables|Private|Camera|SetBaseArmLength (Variables|/Script/Engine.SpringArmComponent|GetTargetArmLength _output_get)))

(fn OnRepPoints
  (Default|CallOnChangedPoints (Variables|Private|Points|GetPoints)))

(fn CalculeMilestoneReachedCamera
  (params (ScaleFactor :type Float%20%28double-precision%29))
  (LocalVariables|SetLocalScaleFactor ScaleFactor)
  (LocalVariables|SetLocalCurrentMilestone (Math|Float|Floor (/ (Variables|Private|Points|GetPoints) 1e+02)))
  (if (> (LocalVariables|GetLocalCurrentMilestone) (Variables|Private|Camera|GetLastMilestone%20))
    (bind _output_get (LocalVariables|SetLocalDelta (- (LocalVariables|GetLocalScaleFactor) 1.0)))
    (bind _output_get_2 (LocalVariables|SetLocalDumping (* _output_get (Variables|Private|Camera|GetCameraGrowthDamping))))
    (Default|CallOnGrowthMilestoneReachedCamera (* (Variables|Private|Camera|GetBaseArmLength) (+ 1.0 _output_get_2)))
    (Variables|Private|Camera|SetLastMilestone%20 (LocalVariables|GetLocalCurrentMilestone))))

(fn CallRemovePoints
  (params (Amount :type Float%20%28double-precision%29) (SmoothRefreshSize :type Boolean))
  (Private|Points|RemovePoints Amount SmoothRefreshSize))

(fn SetShieldActive
  (params (HasActive :type Boolean))
  (Variables|Private|Shield|SetHasShieldActive HasActive))

(fn GetHasShieldActive
  (return (Variables|Private|Shield|GetHasShieldActive)))

(fn IsFullyOverlappingEnemy
  (params (OtherGrowth :type AC%20Growth%20Component%20Object%20Reference))
  (bind _mysphere (Variables|Private|Component|GetMySphere))
  (bind _returnvalue (Components|Sphere|GetScaledSphereRadius _mysphere))
  (LocalVariables|SetLocalOtherSphere (Actor|GetComponentbyClass (Components|GetOwner OtherGrowth) "/Script/Engine.SphereComponent"))
  (if (>= (Math|Float|Clamp(Float) (/ (- (+ (Components|Sphere|GetScaledSphereRadius (LocalVariables|GetLocalOtherSphere)) _returnvalue) (Math|Vector|Distance(Vector) (Transformation|GetWorldLocation (LocalVariables|GetLocalOtherSphere)) (Transformation|GetWorldLocation (Variables|Private|Component|GetMySphere)))) (* _returnvalue 2.0))) 0.8)
    (Development|PrintString "full overlaping" true true "(R=1.000000,G=0.019160,B=0.000000,A=1.000000)" 15.0))
  (return (>= (Math|Float|Clamp(Float) (/ (- (+ (Components|Sphere|GetScaledSphereRadius (LocalVariables|GetLocalOtherSphere)) _returnvalue) (Math|Vector|Distance(Vector) (Transformation|GetWorldLocation (LocalVariables|GetLocalOtherSphere)) (Transformation|GetWorldLocation (Variables|Private|Component|GetMySphere)))) (* _returnvalue 2.0))) 0.8)))

(fn GetCurrentRadius
  (bind _returnvalue (Components|GetOwner))
  (bind _returnvalue_2 (Actor|GetComponentbyClass _returnvalue "/Script/Engine.StaticMeshComponent"))
  (return (* (.X (Math|Vector|BreakVector (.Max (Components|StaticMesh|GetLocalBounds _returnvalue_2)))) (.X (Math|Vector|BreakVector (Transformation|GetWorldScale _returnvalue_2))))))