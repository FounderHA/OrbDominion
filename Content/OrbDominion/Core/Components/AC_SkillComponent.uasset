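; Actor component that manages a player's three single-charge skill slots (Speed, Push, Shield) in OrbDominion.
; TryGrantCharge fills the matching slot if empty, while next/previous selection wraps around to charged slots only, using -1 for none.
; Activation spends the selected charge, runs that skill and advances selection, with dispatchers reporting charge and selection changes.
; Skill effects are placeholders: Speed is empty, while Push and Shield only print.
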(event EventBeginPlay)

(fn TryGrantCharge
  (params (SkillType :type E_SkillType%20Enum :default "NewEnumerator0"))
  (switch Utilities|FlowControl|Switch|SwitchonE_SkillType SkillType
    (:NewEnumerator0
      (LocalVariables|SetTargetIndex 0))
    (:NewEnumerator1
      (LocalVariables|SetTargetIndex 1))
    (:NewEnumerator2
      (LocalVariables|SetTargetIndex 2)))
  (if (not (.HasCharge (Utilities|Struct|BreakS_SkillSlot (Utilities|Array|Get(acopy) (Variables|Default|GetSlots%20) (LocalVariables|GetTargetIndex)))))
    (Utilities|Array|SetArrayElem (Variables|Default|GetSlots%20) (LocalVariables|GetTargetIndex) (Utilities|Struct|MakeS_SkillSlot (.SkillType (Utilities|Struct|BreakS_SkillSlot (Utilities|Array|Get(acopy) (Variables|Default|GetSlots%20) (LocalVariables|GetTargetIndex)))) true))
    (if (== (Variables|Default|GetSelectedIndex%20) -1)
      (Public|SelectNextAvailable))
    (Default|CallOnSkillChargeChanged (LocalVariables|GetTargetIndex) true)
    (return true)
    (else
      (return false))))

(fn SelectNextAvailable
  (bind _index (Utilities|FlowControl|ForLoopwithBreak 0 2 :!label _label)
    (:LoopBody
      (LocalVariables|SetLocalCandidateIndex (Math|Integer|%(Integer) (+ (+ (Variables|Default|GetSelectedIndex%20) _index) 1) 3))
      (if (.hascharge (Utilities|Array|Get(acopy) (Variables|Default|GetSlots%20) (Math|Integer|%(Integer) (+ (+ (Variables|Default|GetSelectedIndex%20) _index) 1) 3)))
        (LocalVariables|SetLocalHasCharge true)
        (bind _output_get (Variables|Default|SetSelectedIndex%20 (LocalVariables|GetLocalCandidateIndex)))
        (Default|CallOnSkillSelected _output_get)
        (goto _label Break)))
    (:Completed
      (if (not (LocalVariables|GetLocalHasCharge))
        (bind _output_get_2 (Variables|Default|SetSelectedIndex%20 -1))
        (Default|CallOnSkillSelected _output_get_2)))))

(fn SelectPreviousAvailable
  (bind _index (Utilities|FlowControl|ForLoopwithBreak 0 2 :!label _label)
    (:LoopBody
      (LocalVariables|SetLocalCandidateIndex (Math|Integer|%(Integer) (+ (- (- (Variables|Default|GetSelectedIndex%20) _index) 1) 9) 3))
      (if (.hascharge (Utilities|Array|Get(acopy) (Variables|Default|GetSlots%20) (Math|Integer|%(Integer) (+ (- (- (Variables|Default|GetSelectedIndex%20) _index) 1) 9) 3)))
        (LocalVariables|SetLocalHasCharge true)
        (bind _output_get (Variables|Default|SetSelectedIndex%20 (LocalVariables|GetLocalCandidateIndex)))
        (Default|CallOnSkillSelected _output_get)
        (goto _label Break)))
    (:Completed
      (if (not (LocalVariables|GetLocalHasCharge))
        (bind _output_get_2 (Variables|Default|SetSelectedIndex%20 -1))
        (Default|CallOnSkillSelected _output_get_2)))))

(fn ActivateSelectedSkill
  (if (not (== (Variables|Default|GetSelectedIndex%20) -1))
    (LocalVariables|SetLocalSkillType (Utilities|Array|Get(acopy) (Variables|Default|GetSlots%20) (Variables|Default|GetSelectedIndex%20)))
    (Utilities|Array|SetArrayElem (Variables|Default|GetSlots%20) (Variables|Default|GetSelectedIndex%20) (Utilities|Struct|MakeS_SkillSlot (Utilities|Struct|BreakS_SkillSlot (LocalVariables|GetLocalSkillType))))
    (Default|CallOnSkillChargeChanged (Variables|Default|GetSelectedIndex%20) false)
    (switch Utilities|FlowControl|Switch|SwitchonE_SkillType (Utilities|Struct|BreakS_SkillSlot (LocalVariables|GetLocalSkillType))
      (:NewEnumerator0
        (Private|Skill|ExecuteSpeedBoost))
      (:NewEnumerator1
        (Private|Skill|ExecutePush))
      (:NewEnumerator2
        (Private|Skill|ExecuteShield)))
    (Public|SelectNextAvailable)))

(fn ExecuteSpeedBoost)

(fn ExecutePush
  (Development|PrintString "push"))

(fn ExecuteShield
  (Development|PrintString "Shield"))