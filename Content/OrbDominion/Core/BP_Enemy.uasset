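; BP_Enemy is an Orb Dominion enemy that wanders between randomly chosen BP_OrbFood actors.
; FindFood runs at BeginPlay and picks a random target from all food actors in the level.
; Tick steers straight at the target with movement input, without pathfinding, and picks again once within AcceptanceRadius.
; With no valid target, Tick retries the search after a delay.
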(event EventBeginPlay
  (|CallParentFunction)
  (CallFunction|FindFood))

(event EventTick
  (params (DeltaSeconds :type Float%20%28single-precision%29))
  (Utilities|IsValid (Variables|Default|GetTargetFood)
    (:Is%20Valid
      (Pawn|Input|AddMovementInput (Math|Vector|GetUnitDirection(Vector) (Transformation|GetActorLocation) (Transformation|GetActorLocation (Variables|Default|GetTargetFood))) 1.0 false)
      (if (<= (Math|Vector|Distance(Vector) (Transformation|GetActorLocation) (Transformation|GetActorLocation (Variables|Default|GetTargetFood))) (Variables|Default|GetAcceptanceRadius))
        (Variables|Default|SetTargetFood 0)
        (CallFunction|FindFood)))
    (:Is%20Not%20Valid
      (Utilities|FlowControl|Delay 1e+01)
      (CallFunction|FindFood))))

(fn ConstructionScript
  (|CallParentFunction))

(fn FindFood
  (bind _outactors (Actor|GetAllActorsOfClass "/Game/OrbDominion/Core/BP_OrbFood.BP_OrbFood_C"))
  (bind _output_get (LocalVariables|SetLocalOrbFoods _outactors))
  (if (Utilities|Array|IsNotEmpty _output_get)
    (Utilities|IsValid (.OutItem (Utilities|Array|Random _output_get))
      (:Is%20Valid
        (Variables|Default|SetTargetFood (.OutItem (Utilities|Array|Random _output_get)))))))