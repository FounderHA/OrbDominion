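; BP_MaterialPreview is a preview object that displays a skin texture on a rotating static mesh for a scene capture.
; BeginPlay creates a dynamic material instance on the mesh and restricts the SceneCaptureComponent2D to that mesh with ShowOnlyComponent.
; Tick spins the mesh in yaw at a constant, frame-rate-independent speed.
; SetPreviewTexture writes the supplied texture into the material's SkinTexture parameter.
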(event Custom|SetPreviewTexture
  (params (SkinTexture :type Texture%202D%20Object%20Reference))
  (Rendering|Material|SetTextureParameterValue (Variables|Default|GetMaterial) "SkinTexture" SkinTexture))

(event EventBeginPlay
  (bind _returnvalue (Rendering|Material|CreateDynamicMaterialInstance (Variables|Default|GetStaticMesh) 0 0 "SkinTexture" :!class /Script/Engine.PrimitiveComponent))
  (Variables|Default|SetMaterial _returnvalue)
  (Rendering|SceneCapture|ShowOnlyComponent (Variables|Default|GetSceneCaptureComponent2D) (Variables|Default|GetStaticMesh)))

(event EventTick
  (params (DeltaSeconds :type Float%20%28single-precision%29))
  (Transformation|AddLocalRotation (Variables|Default|GetStaticMesh) (Math|Rotator|MakeRotator 0.0 0.0 (* DeltaSeconds 3e+01)) false false))

(fn ConstructionScript)