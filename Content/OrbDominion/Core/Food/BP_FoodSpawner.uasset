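; BP_FoodSpawner spawns BP_OrbFood orbs inside a sphere around its own location.
; CallInitialSpawnFood, gated by an Active flag, stores the radius, count and delay, spawns the initial batch and starts a looping timer at the respawn delay.
; SpawnFood uses cube-root random scaling for uniform volume distribution and passes the radius as each orb's TeleportRadius.
; RequestRespawn spawns one more orb.
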(fn ConstructionScript)

(fn CallInitialSpawnFood
  (params (SpawnFoodRadius :type Float%20%28double-precision%29) (InitialSpawnCount :type Integer) (RespawnFoodDelay :type Float%20%28double-precision%29))
  (if (Variables|Private|GetActive)
    (Variables|Private|SetSpawnRadius SpawnFoodRadius)
    (Variables|Private|SetInitialSpawnCount InitialSpawnCount)
    (Variables|Private|SetRespawnFoodDelay RespawnFoodDelay)
    (for _index (range 0 (- (Variables|Private|GetInitialSpawnCount) 1))
      (CallFunction|SpawnFood))
    (bind _returnvalue (Utilities|Time|SetTimerbyEvent (EventDispatchers|CreateEvent :!event RequestRespawn) (Variables|Private|GetRespawnFoodDelay) true))
    (Variables|Private|SetSpawnTimerHandle _returnvalue)))

(fn SpawnFood
  (Game|SpawnActorfromClass "/Game/OrbDominion/Core/Food/BP_OrbFood.BP_OrbFood_C" (Math|Transform|MakeTransform (+ (Transformation|GetActorLocation) (* (Math|Random|RandomUnitVector) (* (Math|Float|Power (Math|Random|RandomFloatinRange 0.0 1.0) 0.3333) (Variables|Private|GetSpawnRadius)))) "0, 0, 0" "1.000000,1.000000,1.000000") "Undefined" "MultiplyWithRoot" 0 (Variables|Private|GetSpawnRadius) 0))

(fn RequestRespawn
  (CallFunction|SpawnFood))