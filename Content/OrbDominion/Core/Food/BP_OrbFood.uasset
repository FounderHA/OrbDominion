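; BP_OrbFood is a food orb pickup that feeds the growth component of actors that touch it.
; On BeginPlay it picks a random entry from ArrayOrbFood to set its value and particle template.
; On sphere overlap it passes the value to FoodAbsorb, fires the OnFoodColected dispatcher and destroys itself.
; TeleportActor, not called here, moves it to a random point within TeleportRadius of world origin.
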(event OnComponentBeginOverlap(Sphere)
  (params (OverlappedComponent :type Primitive%20Component%20Object%20Reference) (OtherActor :type Actor%20Object%20Reference) (OtherComp :type Primitive%20Component%20Object%20Reference) (OtherBodyIndex :type Integer) (bFromSweep :type Boolean) (SweepResult :type Hit%20Result%20Structure%20%28by%20ref%29))
  (bind _ac_growthcomponent (CallFunction|FindGrowthComponent OtherActor))
  (Utilities|IsValid _ac_growthcomponent
    (:Is%20Valid
      (Default|FoodAbsorb _ac_growthcomponent (Variables|Default|GetValue))
      (Default|CallOnFoodColected)
      (Actor|DestroyActor))))

(event EventBeginPlay
  (CallFunction|RandomizeFood))

(fn ConstructionScript)

(fn RandomizeFood
  (bind _arrayorbfood (Variables|Default|GetArrayOrbFood))
  (LocalVariables|SetLocalRandomOrbFood (Utilities|Array|Get(acopy) _arrayorbfood (Math|Random|RandomIntegerinRange 0 (- (Utilities|Array|Length _arrayorbfood) 1))))
  (Variables|Default|SetValue (Variables|/Game/OrbDominion/Core/Data/OrbFood/PDA/PDA_OrbFood.PDA_OrbFood_C|GetValue (LocalVariables|GetLocalRandomOrbFood)))
  (Effects|Components|ParticleSystem|SetTemplate (Variables|Default|GetParticleSystem) (Variables|/Game/OrbDominion/Core/Data/OrbFood/PDA/PDA_OrbFood.PDA_OrbFood_C|GetParticule (LocalVariables|GetLocalRandomOrbFood))))

(fn TeleportActor
  (Transformation|SetActorLocation (+ "" (* (Math|Random|RandomUnitVector) (Math|Random|RandomFloatinRange 0.0 (Variables|Default|GetTeleportRadius)))) false false))