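; Actor component intended to keep its owning pawn inside a spherical dome boundary.
; BeginPlay caches the owner pawn, and SetDomeParameters sets only the radius.
; Helpers compare squared center offset to the full radius, then compute a clamped point inset by the owner's scaled static mesh X extent.
; The check-and-teleport chain is disconnected and Tick is empty, so the boundary is not currently enforced.
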(event EventTick
  (params (DeltaSeconds :type Float%20%28single-precision%29)))

(event EventBeginPlay
  (Private|SetCachedOwnerPawn))

(fn SetDomeParameters
  (params (DomeRadius :type Float%20%28double-precision%29))
  (Variables|Private|SetDomeRadius DomeRadius))

(fn SetOffset
  (params (self2 :type Actor%20Object%20Reference))
  (Variables|Private|SetOffSet (- (Transformation|GetActorLocation self2) (Variables|Private|GetDomeCenter))))

(fn CheckDomeOffSet
  (return (> (Math|Vector|VectorLengthSquared (Variables|Private|GetOffSet)) (Math|Float|Square (Variables|Private|GetDomeRadius)))))

(fn GetDomeClampledLocation
  (bind _output_get (Variables|Private|SetClampedLocation (+ (Variables|Private|GetDomeCenter) (* (Math|Vector|Normalize (Variables|Private|GetOffSet)) (- (Variables|Private|GetDomeRadius) (Private|GetCurrentRadius))))))
  (return _output_get))

(fn SetCachedOwnerPawn
  (bind _aspawn (Utilities|Casting|CastToPawn (Components|GetOwner)))
  (Variables|Private|SetCachedOwnerPawn _aspawn))

(fn GetCurrentRadius
  (bind _returnvalue (Components|GetOwner))
  (bind _returnvalue_2 (Actor|GetComponentbyClass _returnvalue "/Script/Engine.StaticMeshComponent"))
  (return (* (.X (Math|Vector|BreakVector (.Max (Components|StaticMesh|GetLocalBounds _returnvalue_2)))) (.X (Math|Vector|BreakVector (Transformation|GetWorldScale _returnvalue_2))))))