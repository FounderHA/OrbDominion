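; Map configuration actor for the Domo that sets up food spawning when play begins.
; On BeginPlay it reads the DT_MapConfigs row named by MapConfigHandle and caches the food spawn radius and initial count.
; It passes both to the BP_FoodSpawner found in the level to run the initial spawn, or prints a warning if the row is missing.
; Two getters expose the cached values.
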(event EventBeginPlay
  (bind _returnvalue (Utilities|GetDataTableRow "/Game/OrbDominion/Core/Data/DT_MapConfigs.DT_MapConfigs" (.RowName (Utilities|Struct|BreakDataTableRowHandle (Variables|Private|GetMapConfigHandle))))
    (:then
      (Variables|Private|SetSpawnFoodRadius (.SpawnFoodRadius (Utilities|Struct|BreakS_MapConfig _returnvalue)))
      (Variables|Private|SetInitialSpawnCount (.InitialSpawnCount (Utilities|Struct|BreakS_MapConfig _returnvalue)))
      (bind _returnvalue_2 (Actor|GetActorOfClass "/Game/OrbDominion/Core/BP_FoodSpawner.BP_FoodSpawner_C"))
      (Default|CallInitialSpawn _returnvalue_2 (Variables|Private|GetSpawnFoodRadius) (Variables|Private|GetInitialSpawnCount)))
    (:RowNotFound
      (Development|PrintText "Spawn de Food Não Configurado"))))

(fn ConstructionScript)

(fn GetSpawmFoodRadius
  (return (Variables|Private|GetSpawnFoodRadius)))

(fn GetInitialSpawnCount
  (return (Variables|Private|GetInitialSpawnCount)))