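; BP_DomoConfig configures a map at BeginPlay and runs its audio.
; It reads its DT_MapConfigs row, then starts BP_FoodSpawner and BP_SkillSpawner with that row's counts and delays, sharing one spawn radius.
; Random tracks chain through OnAudioFinished until the first player character's growth component reports death, which switches to the EndSimulate sound.
; A missing row only prints a warning, leaving spawners, audio and death binding unstarted.
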(event OnAudioFinished(AudioComponent)
  ;[0.15 0.15 0.15 0.5] Audio Loop
  (if (not (Variables|Default|GetIsPlayerDied))
    (Audio|Components|Audio|SetSound (Variables|Default|GetAudioComponent) (.OutItem (Utilities|Array|Random (Variables|Default|GetAudioArray))))
    (Audio|Components|Audio|Play (Variables|Default|GetAudioComponent) 0.0)))

(event Custom|EventPlayerDie
  ;[0.15 0.15 0.15 0.5] On Player Die
  (Variables|Default|SetIsPlayerDied true)
  (Audio|Components|Audio|SetSound (Variables|Default|GetAudioComponent) "/Engine/EditorSounds/GamePreview/EndSimulate.EndSimulate")
  (Audio|Components|Audio|Play (Variables|Default|GetAudioComponent) 0.0))

(event EventBeginPlay
  (bind _returnvalue (Utilities|GetDataTableRow "/Game/OrbDominion/Core/Data/DT_MapConfigs.DT_MapConfigs" (.RowName (Utilities|Struct|BreakDataTableRowHandle (Variables|Private|GetMapConfigHandle))))
    (:then
      (CallFunction|SetMapConfig _returnvalue)
      (bind _returnvalue_2 (Actor|GetActorOfClass "/Game/OrbDominion/Core/Food/BP_FoodSpawner.BP_FoodSpawner_C"))
      (Default|CallInitialSpawnFood _returnvalue_2 (Variables|Private|GetSpawnRadius) (Variables|Private|GetInitialSpawnFoodCount) (Variables|Private|GetSpawn%20Food%20Delay))
      (bind _returnvalue_3 (Actor|GetActorOfClass "/Game/OrbDominion/Core/Skill/BP_SkillSpawner.BP_SkillSpawner_C"))
      (Default|CallInitialSpawnSkill _returnvalue_3 (Variables|Private|GetSpawnRadius) (Variables|Private|GetInitialSpawnSkillPickupCount) (Variables|Private|GetSpawn%20Skill%20Delay))
      ;[0.15 0.15 0.15 0.5] First Audio
      (Audio|Components|Audio|SetSound (Variables|Default|GetAudioComponent) (.OutItem (Utilities|Array|Random (Variables|Default|GetAudioArray))))
      (Audio|Components|Audio|Play (Variables|Default|GetAudioComponent) 0.0)
      ;[0.15 0.15 0.15 0.5] Bind On Player Die
      (bind _outactors (Actor|GetAllActorsOfClass "/Game/OrbDominion/Player/BP_OrbPlayerCharacter.BP_OrbPlayerCharacter_C"))
      (EventDispatchers|BindEventtoOnPlayerDie (CallFunction|FindGrowthComponent (Utilities|Array|Get(acopy) _outactors)) (EventDispatchers|CreateEvent :!event Custom|EventPlayerDie)))
    (:RowNotFound
      (Development|PrintText "Spawn de Food Não Configurado"))))

(fn ConstructionScript)

(fn GetSpawmFoodRadius
  (return (Variables|Private|GetSpawnRadius)))

(fn GetInitialSpawnCount
  (return (Variables|Private|GetInitialSpawnFoodCount)))

(fn SetMapConfig
  (params (S_MapConfig :type S%20Map%20Config%20Structure%20%28by%20ref%29))
  (bind (_spawnfoodradius _initialspawnfoodcount _initialspawnskillpickupcount _spawnfooddelay _spawnskilldelay) (Utilities|Struct|BreakS_MapConfig S_MapConfig))
  (Variables|Private|SetSpawnRadius _spawnfoodradius)
  (Variables|Private|SetInitialSpawnFoodCount _initialspawnfoodcount)
  (Variables|Private|SetInitialSpawnSkillPickupCount _initialspawnskillpickupcount)
  (Variables|Private|SetSpawn%20Food%20Delay _spawnfooddelay)
  (Variables|Private|SetSpawn%20Skill%20Delay _spawnskilldelay))