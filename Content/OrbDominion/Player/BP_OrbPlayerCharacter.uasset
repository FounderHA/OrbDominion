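; Player-controlled orb pawn for OrbDominion that applies skin, name and control mode from the game instance.
; Enhanced Input drives camera-relative movement, look and skill selection or activation through SkillComponent, while one control mode adds constant forward movement.
; GrowthComponent milestones trigger a timeline that eases camera boom length.
; A looping timer hides distant enemy nameplates and scales nearer ones by distance, and Tick debug-prints max speed.
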(event Custom|GrowthMilestoneCamera
  (params (NewArmLength :type Float%20%28double-precision%29))
  (Private|Camera|ResolveArmLength NewArmLength)
  (bind _alpha (Timeline|TL_CameraZoom PlayFromStart)
    (:Update
      (Variables|/Script/Engine.SpringArmComponent|SetTargetArmLength (Variables|Default|GetCameraBoom) (Math|Float|Lerp (Variables|Private|Camera|GetArmLengthStart%20) (Variables|Private|Camera|GetArmLengthGoal) _alpha)))))

(event Input|EnhancedActionEvents|EnhancedInputActionIA_Move
  (params (ActionValue :type Vector%202D%20Structure) (ElapsedSeconds :type Float%20%28double-precision%29) (TriggeredSeconds :type Float%20%28double-precision%29) (InputAction :type Input%20Action%20Object%20Reference :default "/Game/OrbDominion/Input/Actions/IA_Move.IA_Move"))
  (CallFunction|DoMove ActionValue))

(event Input|EnhancedActionEvents|EnhancedInputActionIA_SkillScroll
  (params (ActionValue :type Float%20%28double-precision%29) (ElapsedSeconds :type Float%20%28double-precision%29) (TriggeredSeconds :type Float%20%28double-precision%29) (InputAction :type Input%20Action%20Object%20Reference :default "/Game/OrbDominion/Input/Actions/IA_SkillScroll.IA_SkillScroll"))
  (Private|Skill|SkillScrollSelector ActionValue))

(event Input|EnhancedActionEvents|EnhancedInputActionIA_MouseLook
  (params (ActionValue :type Vector%202D%20Structure) (ElapsedSeconds :type Float%20%28double-precision%29) (TriggeredSeconds :type Float%20%28double-precision%29) (InputAction :type Input%20Action%20Object%20Reference :default "/Game/OrbDominion/Input/Actions/IA_MouseLook.IA_MouseLook"))
  (Private|Movement|DoLook ActionValue))

(event Input|EnhancedActionEvents|EnhancedInputActionIA_MoveUp
  (params (ActionValue :type Float%20%28double-precision%29) (ElapsedSeconds :type Float%20%28double-precision%29) (TriggeredSeconds :type Float%20%28double-precision%29) (InputAction :type Input%20Action%20Object%20Reference :default "/Game/OrbDominion/Input/Actions/IA_MoveUp.IA_MoveUp"))
  (Private|Movement|DoMoveUp ActionValue))

(event Input|EnhancedActionEvents|EnhancedInputActionIA_SkillActivate
  (params (ActionValue :type Boolean) (ElapsedSeconds :type Float%20%28double-precision%29) (TriggeredSeconds :type Float%20%28double-precision%29) (InputAction :type Input%20Action%20Object%20Reference :default "/Game/OrbDominion/Input/Actions/IA_SkillActivate.IA_SkillActivate"))
  (:Started
    (Default|ActivateSelectedSkill (Variables|Default|GetSkillComponent))))

(event EventBeginPlay
  (|CallParentFunction)
  (Utilities|Time|SetTimerbyFunctionName 0 "SetEnemyNameScale" 0.1 true)
  (Private|Skin|SetSkinandName)
  (Private|Movement|SetControlMode)
  (CallFunction|SetArmLength)
  (EventDispatchers|BindEventtoOnGrowthMilestoneReachedCamera (Variables|Default|GetGrowth%20Component) (EventDispatchers|CreateEvent :!event Custom|GrowthMilestoneCamera))
  (Rendering|SetVisibility (Variables|Default|GetW_OrbName) false false))

(event EventTick
  (params (DeltaSeconds :type Float%20%28single-precision%29))
  (CallFunction|ForwardMove)
  (Development|PrintString (Utilities|String|ToString(Float) (Class|MovementComponent|GetMaxSpeed (Variables|Default|GetFloatingPawnMovement))) true true "(R=0.000000,G=0.660000,B=1.000000,A=1.000000)" 0.0))

(fn ConstructionScript)

(fn ResolveArmLength
  (params (NewArmLength :type Float%20%28double-precision%29))
  (Variables|Private|Camera|SetArmLengthStart%20 (Variables|/Script/Engine.SpringArmComponent|GetTargetArmLength (Variables|Default|GetCameraBoom)))
  (Variables|Private|Camera|SetArmLengthGoal NewArmLength))

(fn DoMove
  (params (InVec :type Vector%202D%20Structure))
  (bind (_x _y) (Math|Vector2D|BreakVector2D InVec))
  (bind _returnvalue (Pawn|GetControlRotation :!class /Script/Engine.Pawn))
  (Pawn|Input|AddMovementInput (Math|Vector|GetForwardVector _returnvalue) _y false)
  (Pawn|Input|AddMovementInput (Math|Vector|GetRightVector (Math|Rotator|MakeRotator 0.0 0.0 (.Yaw (Math|Rotator|BreakRotator _returnvalue)))) _x false))

(fn DoLook
  (params (InVec :type Vector%202D%20Structure))
  (bind (_x _y) (Math|Vector2D|BreakVector2D InVec))
  (Pawn|Input|AddControllerYawInput _x)
  (Pawn|Input|AddControllerPitchInput _y))

(fn DoMoveUp
  (params (ScaleValue :type Float%20%28single-precision%29))
  (Pawn|Input|AddMovementInput "0.000000,0.000000,1.000000" ScaleValue false))

(fn SetControlMode
  (bind _asbp_orb_game_instance (Utilities|Casting|CastToBP_OrbGameInstance (Game|GetGameInstance)))
  (Variables|Private|Movement|SetControlMode (Default|GetControlMode _asbp_orb_game_instance)))

(fn ForwardMove
  (if (Utilities|Enum|Equal(Enum) (Variables|Private|Movement|GetControlMode) "NewEnumerator1")
    (Pawn|Input|AddMovementInput (Math|Vector|GetForwardVector (Pawn|GetControlRotation :!class /Script/Engine.Pawn)) 1.0 false)))

(fn SetSkinandName
  (bind _asbp_orb_game_instance (Utilities|Casting|CastToBP_OrbGameInstance (Game|GetGameInstance)))
  (Rendering|Material|SetTextureParameterValue (Variables|Default|GetPlayerSkinDMI) "SkinTexture" (Variables|/Game/OrbDominion/Core/BP_OrbGameInstance.BP_OrbGameInstance_C|GetSkinTexture _asbp_orb_game_instance))
  (Variables|Default|SetOrbName (Variables|/Game/OrbDominion/Core/BP_OrbGameInstance.BP_OrbGameInstance_C|GetOrbName _asbp_orb_game_instance))
  (bind _aswbp_nameplate (Utilities|Casting|CastToWBP_Nameplate (UserInterface|GetWidget (Variables|Default|GetW_OrbName))))
  (Default|SetOrbName _aswbp_nameplate (Variables|Default|GetOrbName)))

(fn SetArmLength
  (Variables|Private|Camera|SetArmLengthGoal (Variables|/Script/Engine.SpringArmComponent|GetTargetArmLength (Variables|Default|GetCameraBoom))))

(fn SkillScrollSelector
  (params (A :type Float%20%28double-precision%29))
  (bind _skillcomponent (Variables|Default|GetSkillComponent))
  (if (> A 0.0)
    (Default|SelectNextAvailable _skillcomponent)
    (else
      (Default|SelectPreviousAvailable _skillcomponent))))

(fn SetEnemyNameScale
  (if (Pawn|IsLocallyControlled)
    (bind _outactors (Actor|GetAllActorsOfClass "/Game/OrbDominion/Enemy/BP_Enemy.BP_Enemy_C"))
    (for _array_element _outactors
      (bind _output_get (LocalVariables|SetLocalWOrbName (Variables|/Game/OrbDominion/Core/BP_OrbBasePawn.BP_OrbBasePawn_C|GetW_OrbName _array_element)))
      (Utilities|IsValid _output_get
        (:Is%20Valid
          (if (> (Math|Float|Absolute(Float) (Math|Vector|VectorLength (- (Transformation|GetActorLocation _array_element) (Transformation|GetActorLocation self)))) 5e+03)
            (Rendering|SetVisibility (LocalVariables|GetLocalWOrbName) false false)
            (else
              (Rendering|SetVisibility (LocalVariables|GetLocalWOrbName) true false)
              (Widget|Transform|SetRenderScale (Variables|/Game/OrbDominion/UI/Player/WBP_Nameplate.WBP_Nameplate_C|GetSizeBox (.AsWBP%20Nameplate (Utilities|Casting|CastToWBP_Nameplate (UserInterface|GetWidget (LocalVariables|GetLocalWOrbName))))) (Math|Conversions|ToVector2D(Vector) (- 1.0 (Math|Float|MapRangeClamped (Math|Float|Absolute(Float) (Math|Vector|VectorLength (- (Transformation|GetActorLocation _array_element) (Transformation|GetActorLocation self)))) 1e+03 8e+03 0.0 1.0)))))))))))