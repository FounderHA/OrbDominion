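; BP_OrbPlayerController is the player controller for OrbDominion that sets up input and cursor state when play begins.
; It reads the control mode from BP_OrbGameInstance and adds the matching Enhanced Input mapping context, either default or auto-forward, each paired with a shared mouse-look context.
; It then switches to game-only input and hides the mouse cursor.
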(event EventBeginPlay
  (Private|AddMappingInput)
  (Input|SetInputModeGameOnly self false)
  (Variables|Default|SetbShowMouseCursor false))

(fn ConstructionScript)

(fn AddMappingInput
  (bind _asbp_orb_game_instance (Utilities|Casting|CastToBP_OrbGameInstance (Game|GetGameInstance)))
  (bind _output_get (Variables|Private|SetControlMode (Default|GetControlMode _asbp_orb_game_instance)))
  (switch Utilities|FlowControl|Switch|SwitchonE_ControlMode _output_get
    (:NewEnumerator0
      (Input|AddMappingContext (PlayerController|LocalPlayerSubsystems|GetEnhancedInputLocalPlayerSubsystem self) "/Game/OrbDominion/Input/IMC_DefaultMode.IMC_DefaultMode" 0 "(bIgnoreAllPressedKeysUntilRelease=True,bForceImmediately=False,bNotifyUserSettings=False)")
      (Input|AddMappingContext (PlayerController|LocalPlayerSubsystems|GetEnhancedInputLocalPlayerSubsystem self) "/Game/OrbDominion/Input/IMC_MouseLook.IMC_MouseLook" 0 "(bIgnoreAllPressedKeysUntilRelease=True,bForceImmediately=False,bNotifyUserSettings=False)"))
    (:NewEnumerator1
      (Input|AddMappingContext (PlayerController|LocalPlayerSubsystems|GetEnhancedInputLocalPlayerSubsystem self) "/Game/OrbDominion/Input/IMC_ForwardMode.IMC_ForwardMode" 0 "(bIgnoreAllPressedKeysUntilRelease=True,bForceImmediately=False,bNotifyUserSettings=False)")
      (Input|AddMappingContext (PlayerController|LocalPlayerSubsystems|GetEnhancedInputLocalPlayerSubsystem self) "/Game/OrbDominion/Input/IMC_MouseLook.IMC_MouseLook" 0 "(bIgnoreAllPressedKeysUntilRelease=True,bForceImmediately=False,bNotifyUserSettings=False)"))))